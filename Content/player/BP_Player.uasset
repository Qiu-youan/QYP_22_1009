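; Player character Blueprint that handles movement, look, jumping and interaction with world objects through Enhanced Input, adding the default mapping context on BeginPlay.
; Interact runs four separate debug-drawn line traces from the camera along control rotation, each casting to one type: display case, door, small sphere or exit door.
; A successful cast calls that actor's Interact, and the small sphere also sets the Bfan3done flag.
; Some disconnected test and interaction nodes remain unused.
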(event Input|EnhancedActionEvents|EnhancedInputActionIA_move
  (params (ActionValue :type Vector%202D%20Structure) (ElapsedSeconds :type Float%20%28double-precision%29) (TriggeredSeconds :type Float%20%28double-precision%29) (InputAction :type Input%20Action%20Object%20Reference :default "/Game/player/IA/IA_move.IA_move"))
  (bind (_x _y) (Math|Vector2D|BreakVector2D ActionValue))
  (bind _returnvalue (Pawn|GetControlRotation :!class /Script/Engine.Pawn))
  (Pawn|Input|AddMovementInput (+ (* _x (Math|Vector|GetForwardVector _returnvalue)) (* _y (Math|Vector|GetRightVector _returnvalue))) 1.0 false))

(event Input|EnhancedActionEvents|EnhancedInputActionIA_look
  (params (ActionValue :type Vector%202D%20Structure) (ElapsedSeconds :type Float%20%28double-precision%29) (TriggeredSeconds :type Float%20%28double-precision%29) (InputAction :type Input%20Action%20Object%20Reference :default "/Game/player/IA/IA_look.IA_look"))
  (Pawn|Input|AddControllerPitchInput (.Y (Math|Vector2D|BreakVector2D ActionValue))))

(event Input|EnhancedActionEvents|EnhancedInputActionIA_look
  (params (ActionValue :type Vector%202D%20Structure) (ElapsedSeconds :type Float%20%28double-precision%29) (TriggeredSeconds :type Float%20%28double-precision%29) (InputAction :type Input%20Action%20Object%20Reference :default "/Game/player/IA/IA_look.IA_look"))
  (Pawn|Input|AddControllerYawInput (.X (Math|Vector2D|BreakVector2D ActionValue))))

(event Input|EnhancedActionEvents|EnhancedInputActionIA_interact
  (params (ActionValue :type Boolean) (ElapsedSeconds :type Float%20%28double-precision%29) (TriggeredSeconds :type Float%20%28double-precision%29) (InputAction :type Input%20Action%20Object%20Reference :default "/Game/player/IA/IA_interact.IA_interact"))
  (bind _returnvalue (Game|GetPlayerCameraManager 0))
  (bind _returnvalue_2 (Camera|GetCameraLocation _returnvalue))
  (:Started
    (bind _outhit (Collision|LineTraceByChannel _returnvalue_2 (+ _returnvalue_2 (* (Math|Vector|GetForwardVector (Pawn|GetControlRotation :!class /Script/Engine.Pawn)) 2e+03)) "TraceTypeQuery1" false 0 "ForOneFrame"))
    (bind _asbp_exitdoor (Utilities|Casting|CastToBP_Exitdoor (.HitActor (Collision|BreakHitResult _outhit))))
    (Default|Interact _asbp_exitdoor)))

(event Input|EnhancedActionEvents|EnhancedInputActionIA_interact
  (params (ActionValue :type Boolean) (ElapsedSeconds :type Float%20%28double-precision%29) (TriggeredSeconds :type Float%20%28double-precision%29) (InputAction :type Input%20Action%20Object%20Reference :default "/Game/player/IA/IA_interact.IA_interact"))
  (bind _returnvalue (Game|GetPlayerCameraManager 0))
  (bind _returnvalue_2 (Camera|GetCameraLocation _returnvalue))
  (:Started
    (bind _outhit (Collision|LineTraceByChannel _returnvalue_2 (+ _returnvalue_2 (* (Math|Vector|GetForwardVector (Pawn|GetControlRotation :!class /Script/Engine.Pawn)) 2e+03)) "TraceTypeQuery1" false 0 "ForOneFrame"))
    (bind _asbp_displaycase (Utilities|Casting|CastToBP_displaycase (.HitActor (Collision|BreakHitResult _outhit))))
    (Default|Interact _asbp_displaycase)))

(event Input|EnhancedActionEvents|EnhancedInputActionIA_jump
  (params (ActionValue :type Boolean) (ElapsedSeconds :type Float%20%28double-precision%29) (TriggeredSeconds :type Float%20%28double-precision%29) (InputAction :type Input%20Action%20Object%20Reference :default "/Game/player/IA/IA_jump.IA_jump"))
  (:Started
    (Character|Jump))
  (:Completed
    (Character|StopJumping)))

(event Input|EnhancedActionEvents|EnhancedInputActionIA_interact
  (params (ActionValue :type Boolean) (ElapsedSeconds :type Float%20%28double-precision%29) (TriggeredSeconds :type Float%20%28double-precision%29) (InputAction :type Input%20Action%20Object%20Reference :default "/Game/player/IA/IA_interact.IA_interact"))
  (bind _returnvalue (Game|GetPlayerCameraManager 0))
  (bind _returnvalue_2 (Camera|GetCameraLocation _returnvalue))
  (:Started
    (bind _outhit (Collision|LineTraceByChannel _returnvalue_2 (+ _returnvalue_2 (* (Math|Vector|GetForwardVector (Pawn|GetControlRotation :!class /Script/Engine.Pawn)) 2e+03)) "TraceTypeQuery1" false 0 "ForOneFrame"))
    (bind _asbp_door_1 (Utilities|Casting|CastToBP_door1 (.HitActor (Collision|BreakHitResult _outhit))))
    (Default|Interact _asbp_door_1)))

(event Input|EnhancedActionEvents|EnhancedInputActionIA_interact
  (params (ActionValue :type Boolean) (ElapsedSeconds :type Float%20%28double-precision%29) (TriggeredSeconds :type Float%20%28double-precision%29) (InputAction :type Input%20Action%20Object%20Reference :default "/Game/player/IA/IA_interact.IA_interact"))
  (bind _returnvalue (Game|GetPlayerCameraManager 0))
  (bind _returnvalue_2 (Camera|GetCameraLocation _returnvalue))
  (:Started
    (bind _outhit (Collision|LineTraceByChannel _returnvalue_2 (+ _returnvalue_2 (* (Math|Vector|GetForwardVector (Pawn|GetControlRotation :!class /Script/Engine.Pawn)) 2e+03)) "TraceTypeQuery1" false 0 "ForOneFrame"))
    (bind _asbp_smallsphere (Utilities|Casting|CastToBP_Smallsphere (.HitActor (Collision|BreakHitResult _outhit))))
    (Default|Interact _asbp_smallsphere)
    (Variables|Default|Setbfan3done true)))

(event EventBeginPlay
  (Input|AddMappingContext (PlayerController|LocalPlayerSubsystems|GetEnhancedInputLocalPlayerSubsystem (Game|GetPlayerController 0)) "/Game/player/IA/IMC_default.IMC_default" 0 "(bIgnoreAllPressedKeysUntilRelease=True,bForceImmediately=False,bNotifyUserSettings=False)"))

(event Collision|EventActorBeginOverlap
  (params (OtherActor :type Actor%20Object%20Reference)))

(event EventTick
  (params (DeltaSeconds :type Float%20%28single-precision%29)))

(fn ConstructionScript)