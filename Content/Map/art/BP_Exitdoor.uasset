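; BP_Exitdoor is an exit door that stays locked until the player has collected enough coins and completed enough case and projection interactions.
; Interact casts the player character to BP_Player and compares its Coin, Case and Projection counts against fixed thresholds.
; When all are met, a FlipFlop plays or reverses the DoorAnim timeline, rotating DoorPivot between closed and open.
; Otherwise it prints the current counts and a Chinese locked-door message to the screen.
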(event Custom|Interact
  (bind _asbp_player (Utilities|Casting|CastToBP_Player (Game|GetPlayerCharacter 0)))
  (if (Math|Boolean|ANDBoolean (>= (Variables|/Game/player/BP_Player.BP_Player_C|GetCoinCount _asbp_player) 9) (>= (Variables|/Game/player/BP_Player.BP_Player_C|GetCaseCount _asbp_player) 3) (>= (Variables|/Game/player/BP_Player.BP_Player_C|GetProjectionCount _asbp_player) 6))
    (Utilities|FlowControl|FlipFlop
      (:A
        (bind _alpha (Timeline|doorAnim Play)
          (:Update
            (Transformation|SetRelativeRotation (Variables|Default|Getdoor%20pivot) (Math|Rotator|Lerp(Rotator) "0, 0, 0" "0.000000,90.000000,0.000000" _alpha) false false))))
      (:B
        (Timeline|doorAnim Reverse)))
    (else
      (Development|PrintString (Utilities|String|ToString(Text) (Utilities|Text|FormatText "Coin:{0} Case:{1} Projection:{2}" (Variables|/Game/player/BP_Player.BP_Player_C|GetCoinCount _asbp_player) (Variables|/Game/player/BP_Player.BP_Player_C|GetCaseCount _asbp_player) (Variables|/Game/player/BP_Player.BP_Player_C|GetProjectionCount _asbp_player))))
      (Development|PrintString "大门已锁死，必须完成所有展厅交互并找到古币才能开启！"))))

(event EventBeginPlay)

(event Collision|EventActorBeginOverlap
  (params (OtherActor :type Actor%20Object%20Reference)))

(event EventTick
  (params (DeltaSeconds :type Float%20%28single-precision%29)))

(fn ConstructionScript)