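; BP_projectionPlatform is a map actor that reveals a painting on a plane while the player stands inside its trigger box.
; On box overlap by BP_Player, it increments that player's ProjectionCount, shows the Plane and applies the MyPainting material to it.
; When the player leaves the box, the Plane is hidden again, while the count is not decremented, so repeat entries keep adding to it.
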(event OnComponentBeginOverlap(Box)
  (params (OverlappedComponent :type Primitive%20Component%20Object%20Reference) (OtherActor :type Actor%20Object%20Reference) (OtherComp :type Primitive%20Component%20Object%20Reference) (OtherBodyIndex :type Integer) (bFromSweep :type Boolean) (SweepResult :type Hit%20Result%20Structure%20%28by%20ref%29))
  (bind _asbp_player (Utilities|Casting|CastToBP_Player OtherActor))
  (Variables|/Game/player/BP_Player.BP_Player_C|SetProjectionCount _asbp_player (+ (Variables|/Game/player/BP_Player.BP_Player_C|GetProjectionCount _asbp_player) 1))
  (Rendering|SetVisibility (Variables|Default|GetPlane) true false)
  (Rendering|Material|SetMaterial (Variables|Default|GetPlane) 0 (Variables|Default|GetMyPainting)))

(event OnComponentEndOverlap(Box)
  (params (OverlappedComponent :type Primitive%20Component%20Object%20Reference) (OtherActor :type Actor%20Object%20Reference) (OtherComp :type Primitive%20Component%20Object%20Reference) (OtherBodyIndex :type Integer))
  (Utilities|Casting|CastToBP_Player OtherActor)
  (Rendering|SetVisibility (Variables|Default|GetPlane) false false))

(event EventBeginPlay)

(event Collision|EventActorBeginOverlap
  (params (OtherActor :type Actor%20Object%20Reference)))

(event EventTick
  (params (DeltaSeconds :type Float%20%28single-precision%29)))

(fn ConstructionScript)