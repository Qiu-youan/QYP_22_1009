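; Interactive display case actor whose glass lowers to expose a collectible exhibit.
; Interact alternately plays and reverses a timeline that slides the glass, and increments the player's CaseCount on every use.
; Finishing the timeline enables the exhibit trigger, where player overlap hides the exhibit once and increments CaseCount again.
; The exhibit mesh is assigned from a variable at BeginPlay.
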(event OnComponentBeginOverlap(ExhibitTrigger)
  (params (OverlappedComponent :type Primitive%20Component%20Object%20Reference) (OtherActor :type Actor%20Object%20Reference) (OtherComp :type Primitive%20Component%20Object%20Reference) (OtherBodyIndex :type Integer) (bFromSweep :type Boolean) (SweepResult :type Hit%20Result%20Structure%20%28by%20ref%29))
  (bind _asbp_player (Utilities|Casting|CastToBP_Player OtherActor))
  (if (not (Variables|Default|GetbIsPickedUp))
    (Variables|/Game/player/BP_Player.BP_Player_C|SetCaseCount _asbp_player (+ (Variables|/Game/player/BP_Player.BP_Player_C|GetCaseCount _asbp_player) 1))
    (Rendering|SetVisibility (Variables|Default|GetExnibit) false false)
    (Collision|SetCollisionEnabled (Variables|Default|GetExhibitTrigger) "NoCollision")
    (Variables|Default|SetbIsPickedUp true)))

(event Custom|Interact
  (Utilities|FlowControl|Sequence
    (:then_0
      (Utilities|FlowControl|FlipFlop
        (:A
          (bind _alpha (Timeline|caseanim Play)
            (:Update
              (Transformation|SetRelativeLocation (Variables|Default|Getglassroot) (Math|Vector|Lerp(Vector) "0.000000,0.000000,20.000000" "0.000000,0.000000,-200.000000" _alpha) false false))
            (:Finished
              (Collision|SetCollisionEnabled (Variables|Default|GetExhibitTrigger) "QueryOnly")
              (Variables|Default|SetbTsGlassDown true))))
        (:B
          (Timeline|caseanim Reverse))))
    (:then_1
      (bind _asbp_player (Utilities|Casting|CastToBP_Player (Game|GetPlayerCharacter 0)))
      (Variables|/Game/player/BP_Player.BP_Player_C|SetCaseCount _asbp_player (+ (Variables|/Game/player/BP_Player.BP_Player_C|GetCaseCount _asbp_player) 1)))))

(event Collision|EventActorBeginOverlap
  (params (OtherActor :type Actor%20Object%20Reference)))

(event EventTick
  (params (DeltaSeconds :type Float%20%28single-precision%29)))

(event EventBeginPlay
  (Components|StaticMesh|SetStaticMesh (Variables|Default|GetExnibit) (Variables|Default|GetExhibitMeshAsset)))

(fn ConstructionScript)